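; Actor that plays a reversible disappear effect around its location, toggled by a bound trigger, with reverse running at triple speed.
; A timeline drives DisappearAnimate, which shrinks a radius in MPC_Disappear and sets burn color, burn scale and direction-dependent Niagara ring, spawn and attraction parameters.
; It also blends post-process and crossfades sunlight to an alien light.
; On BeginPlay, a cube scene capture renders only the skysphere to a render target.
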(event Custom|Toggle%20Disappear
  (params (Animate :type Boolean) (Direction :type ETimelineDirection%20Enum :default "Forward"))
  ;[1 1 1] Animate disappear effect - forward and reverse
  (if Animate
    (Variables|Default|SetCustomTimeDilation 1.0)
    (switch Utilities|FlowControl|Switch|SwitchonETimelineDirection Direction
      (:Forward
        (bind (_direction _disappeartime) (Timeline|Timeline Play)
          (:Update
            (CallFunction|DisappearAnimate _direction _disappeartime))))
      (:Backward
        (Variables|Default|SetCustomTimeDilation 3.0)
        (Timeline|Timeline Reverse)))
    (else
      (Timeline|Timeline Stop))))

(event EventBeginPlay
  (EventDispatchers|BindEventtoButtonToggled (Variables|Setup|GetTriggerBP) (delegate Custom|Toggle%20Disappear))
  (Variables|Setup|SetDisappearValue 0.0)
  (CallFunction|Initialize)
  (CallFunction|CaptureSky))

(fn ConstructionScript
  (CallFunction|Initialize))

(fn Initialize
  (Rendering|Material|SetVectorParameterValue "/Game/Disappear/MPC_Disappear.MPC_Disappear" "DisappearCenter" (Math|Conversions|ToLinearColor(Vector) (Transformation|GetWorldLocation (Variables|Default|GetDefaultSceneRoot))) :!class /Script/Engine.KismetMaterialLibrary)
  (Transformation|SetRelativeScale3D (Variables|Default|GetSM_SkyboxBurn) (Math|Conversions|ToVector(Float) (/ (Variables|Setup|GetSkysphereRadius) 1e+02)))
  (CallFunction|DisappearAnimate "Forward" (Variables|Setup|GetDisappearValue)))

(fn CaptureSky
  (CallFunction|DisappearAnimate "Forward" 0.0)
  (Variables|/Script/Engine.SceneCaptureComponent|SetShowOnlyActors (Variables|Default|GetSceneCaptureComponentCube) (Variables|Setup|GetSkysphere))
  (Rendering|SceneCapture|CaptureScene (Variables|Default|GetSceneCaptureComponentCube) :!class /Script/Engine.SceneCaptureComponentCube)
  (Development|PrintString "Disappear: Captured sky into RenderTarget" false))

(fn DisappearAnimate
  (params (Direction :type ETimelineDirection%20Enum :default "Forward") (DisappearValue :type Float%20%28single-precision%29))
  (LocalVariables|SetL_Direction Direction)
  (LocalVariables|SetL_DisappearValue DisappearValue)
  (LocalVariables|SetL_DisappearRadius (Math|Float|MapRangeClamped (LocalVariables|GetL_DisappearValue) 0.0 1.0 (Variables|Setup|GetDisappearMaxRadius) (Variables|Setup|GetDisappearMinRadius)))
  (Utilities|FlowControl|Sequence
    (:then_0
      ;[1 1 1] Direction
      (Niagara|SetNiagaraVariable(Float) (Variables|Default|GetNiagara) "AttractionStrength" (Utilities|Select :Index (LocalVariables|GetL_Direction) :Forward 0.0 :Backward 15.0))
      (Niagara|SetNiagaraVariable(Float) (Variables|Default|GetNiagara) "KillRadius" (Utilities|Select :Index (LocalVariables|GetL_Direction) :Forward 0.0 :Backward (LocalVariables|GetL_DisappearRadius)))
      (Rendering|Material|SetVectorParameterValue "/Game/Disappear/MPC_Disappear.MPC_Disappear" "BurnColor" (Math|Color|SelectColor "(R=19.270802,G=25.829393,B=100.000000,A=1.000000)" "(R=3.854159,G=20.000000,B=14.079859,A=1.000000)" (Utilities|Select :Index (LocalVariables|GetL_Direction) :Forward true :Backward false)) :!class /Script/Engine.KismetMaterialLibrary))
    (:then_1
      ;[1 1 1] NIagara by radius
      (Rendering|Material|SetScalarParameterValue "/Game/Disappear/MPC_Disappear.MPC_Disappear" "DisappearRadius" (LocalVariables|GetL_DisappearRadius) :!class /Script/Engine.KismetMaterialLibrary)
      (Niagara|SetNiagaraVariable(Float) (Variables|Default|GetNiagara) "RingRadius" (+ (LocalVariables|GetL_DisappearRadius) (+ (Variables|Default|GetNiagaraRadiusOffset) (Utilities|Select :Index (LocalVariables|GetL_Direction) :Forward 0.0 :Backward 5e+02))))
      (Rendering|Material|SetScalarParameterValue "/Game/Disappear/MPC_Disappear.MPC_Disappear" "BurnScale" (Math|Float|MapRangeClamped (LocalVariables|GetL_DisappearValue) 0.54 0.55 5.0 1.0) :!class /Script/Engine.KismetMaterialLibrary))
    (:then_2
      ;[1 1 1] Niagara
      (Rendering|SetVisibility (Variables|Default|GetNiagara) (>= (LocalVariables|GetL_DisappearValue) 0.1) false)
      (Niagara|SetNiagaraVariable(Float) (Variables|Default|GetNiagara) "SpawnRateSky" (Math|Float|MapRangeClamped (LocalVariables|GetL_DisappearValue) 0.3 0.4 1e+03 0.0))
      (Niagara|SetNiagaraVariable(Float) (Variables|Default|GetNiagara) "SpawnRate" (Math|Float|MapRangeClamped (LocalVariables|GetL_DisappearValue) 0.5 1.0 5e+02 1e+02)))
    (:then_3
      ;[1 1 1] PostProcess
      (Variables|/Script/Engine.PostProcessComponent|SetBlendWeight (Variables|Default|GetPostProcessLighting) (Math|Float|MapRangeClamped (LocalVariables|GetL_DisappearValue) 0.0 0.5 0.0 1.0))
      (Rendering|Components|Light|SetIntensity (Variables|/Script/Engine.Light|GetLightComponent (Variables|Setup|GetSunLight)) (Math|Float|MapRangeClamped (LocalVariables|GetL_DisappearValue) 0.0 1.0 (Variables|Default|GetSunLightIntensity) 0.0))
      (Rendering|Components|Light|SetIntensity (Variables|Default|GetDirectionalLightAlien) (Math|Float|MapRangeClamped (LocalVariables|GetL_DisappearValue) 0.0 1.0 0.0 (Variables|Default|GetSunLightAlienIntensity))))))