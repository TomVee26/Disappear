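; BP_Disappear_Trigger is a button trigger that toggles when something enters or leaves its TriggerVolume.
; Both overlap events share a FlipFlop that plays or reverses a Timeline, blending the button's color between grey and blue through a dynamic material instance created in the Construction Script.
; Every Timeline update also calls the ButtonToggled dispatcher with the FlipFlop state, so it fires repeatedly during each transition.
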(event OnComponentBeginOverlap(TriggerVolume)
  (params (OverlappedComponent :type Primitive%20Component%20Object%20Reference) (OtherActor :type Actor%20Object%20Reference) (OtherComp :type Primitive%20Component%20Object%20Reference) (OtherBodyIndex :type Integer) (bFromSweep :type Boolean) (SweepResult :type Hit%20Result%20Structure%20%28by%20ref%29))
  (bind _isa (Utilities|FlowControl|FlipFlop)
    (:A
      (bind _buttonactivate (Timeline|Timeline Play)
        (:Update
          (Rendering|Material|SetVectorParameterValue (Variables|Default|GetButtonColorDMI) "Color" (Math|Color|Lerp(LinearColor) "(R=0.359375,G=0.359375,B=0.359375,A=1.000000)" "(R=0.000000,G=0.294383,B=1.000000,A=1.000000)" _buttonactivate) :!class /Script/Engine.MaterialInstanceDynamic)
          (Default|CallButtonToggled _isa))))
    (:B
      (Timeline|Timeline Reverse))))

(event OnComponentEndOverlap(TriggerVolume)
  (params (OverlappedComponent :type Primitive%20Component%20Object%20Reference) (OtherActor :type Actor%20Object%20Reference) (OtherComp :type Primitive%20Component%20Object%20Reference) (OtherBodyIndex :type Integer))
  (bind _isa (Utilities|FlowControl|FlipFlop)
    (:A
      (bind _buttonactivate (Timeline|Timeline Play)
        (:Update
          (Rendering|Material|SetVectorParameterValue (Variables|Default|GetButtonColorDMI) "Color" (Math|Color|Lerp(LinearColor) "(R=0.359375,G=0.359375,B=0.359375,A=1.000000)" "(R=0.000000,G=0.294383,B=1.000000,A=1.000000)" _buttonactivate) :!class /Script/Engine.MaterialInstanceDynamic)
          (Default|CallButtonToggled _isa))))
    (:B
      (Timeline|Timeline Reverse))))

(fn ConstructionScript
  (bind _returnvalue (Rendering|Material|CreateDynamicMaterialInstance (Variables|Default|GetButton) 0 0 "ButtonColor" :!class /Script/Engine.PrimitiveComponent))
  (Variables|Default|SetButtonColorDMI _returnvalue))